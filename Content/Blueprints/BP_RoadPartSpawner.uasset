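; BP_RoadPartSpawner builds an endless road that extends along negative X as the player advances.
; On BeginPlay it lays an initial run of static mesh components, placing each at a fixed spacing from an incrementing section counter.
; When the player overlaps the trigger Box, the Box jumps one section forward, a new part is appended and the oldest is destroyed.
; Despite its name, AddRandomRoadPart contains no random selection.
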(event OnComponentBeginOverlap(Box)
  (params (OverlappedComponent :type Primitive%20Component%20Object%20Reference) (OtherActor :type Actor%20Object%20Reference) (OtherComp :type Primitive%20Component%20Object%20Reference) (OtherBodyIndex :type Integer) (bFromSweep :type Boolean) (SweepResult :type Hit%20Result%20Structure%20%28by%20ref%29))
  (if (== OtherActor (Game|GetPlayerCharacter 0))
    (Transformation|AddRelativeLocation (Variables|Default|GetBox) "-5000.000000,0.000000,0.000000" false false)
    (CallFunction|AddRandomRoadPart)
    (Components|DestroyComponent (Utilities|Array|Get(acopy) (Variables|Default|GetAllRoadParts)))
    (Utilities|Array|RemoveIndex (Variables|Default|GetAllRoadParts))))

(event EventBeginPlay
  (for _index (range 0 6)
    (CallFunction|AddRandomRoadPart)))

(fn ConstructionScript)

(fn AddRandomRoadPart
  (bind _result (Math|Integer|IncrementInt (Variables|Default|GetSectionCounter))
    (:%20%20
      (bind _returnvalue (AddComponent|AddStaticMeshComponent false (Math|Transform|MakeTransform (Math|Vector|MakeVector (Math|Conversions|ToFloat(Integer) (* _result -5000)) 0.0 0.0))))
      (Utilities|Array|Add (Variables|Default|GetAllRoadParts) _returnvalue))))